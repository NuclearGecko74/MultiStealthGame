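; BP_BlackHole is a short-lived black hole actor in the Challenges content that destroys itself five seconds after BeginPlay.
; Every Tick it fires its RadialForce component's impulse to act on nearby objects.
; When an actor begins overlapping Sphere1, it is destroyed if it is exactly a BP_Guard or if its static mesh component is simulating physics.
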(event `self.ReceiveBeginPlay`
  (`KismetSystemLibrary.Delay` 5.0)
  (`self.K2_DestroyActor`))

(event `self.ReceiveTick`
  (params (DeltaSeconds :type "Float (single-precision)"))
  (`RadialForceComponent.FireImpulse` (`self.RadialForce`)))

(event `self.Sphere1.OnComponentBeginOverlap`
  (params (OverlappedComponent :type "PrimitiveComponent Object Reference") (OtherActor :type "Actor Object Reference") (OtherComp :type "PrimitiveComponent Object Reference") (OtherBodyIndex :type Integer) (bFromSweep :type Boolean) (SweepResult :type "HitResult Structure (by ref)"))
  (if (== (`GameplayStatics.GetObjectClass` OtherActor) "/Game/Blueprints/BP_Guard.BP_Guard_C")
    (`self.K2_DestroyActor` OtherActor)
    (elif (`SceneComponent.IsSimulatingPhysics` (`self.GetComponentByClass` OtherActor "/Script/Engine.StaticMeshComponent") "None")
      (`self.K2_DestroyActor` OtherActor))))

(fn `UserConstructionScript`)